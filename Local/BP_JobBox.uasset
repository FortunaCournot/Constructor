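; BP_JobBox is a box actor that replaces itself with the building matching a building item put into its inventory.
; On the server it listens for added items and looks up the item's template ID in ItemTable for the building class.
; It spawns that class at its mesh transform with the same owner, bypassing blocker volumes, and assigns a unique ID and flags persistence dirty.
; After a debug print, it removes the item and destroys itself.
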(event `self.ReceiveBeginPlay`
  (`parent.ReceiveBeginPlay`)
  (if (`KismetSystemLibrary.IsServer`)
    (add `ItemInventory.SignalItemAdded` (`self.PlaceableInventory`) (delegate `OnItemAdded`))))

(event `OnItemAdded`
  (params (index :type Integer) (item :type "GameItem Object Reference") (srcInventory :type "ItemInventory Object Reference") (srcIndex :type Integer))
  (bind _asbuilding_item (cast `BuildingItem` item))
  (bind _templateid (`GameItem.TemplateID` _asbuilding_item))
  (bind _returnvalue (`|GetDataTableRow` "/Game/Items/ItemTable.ItemTable" (`KismetStringLibrary.Conv_StringToName` (`KismetStringLibrary.Conv_IntToString` _templateid)))
    (:`then`
      (bind (_name _shortdesc _longdesc _icon _itemclass _buildingclass _visualobject _actionblueprint_use _maxstacksize _equiplocation _guicategory _itemtags _armourvalue _armortype _soundphysicalsurface _weapontype _weaponarchetype _compatableammunitions _soundtransmittertype _knockbackresponseweapon _weaponstaminaattacksinglebasic _weaponstaminaattacksinglespecial _weaponstaminaattackdualbasic _weaponstaminaattackdualspecial _weaponstaminaheavychargedregenmodifier _weaponspeedheavychargedmodifier _encumbranceweight _coneangle _conemaxdistance _damagehealthlight_onhit _damagehealthheavy_onhit _damagestaminalight_onhit _damagestaminaheavy_onhit _damagehealthlight_onblock _damagehealthheavy_onblock _damagestaminalight_onblock _damagestaminaheavy_onblock _harvestdamage _weaponusage _maxattackreach _minattackreach _minattackdistance _weaponeffectwidth _weaponeffectheight _itemtier _armorpen _damageconcussivelightonhit _damageconcussiveheavyonhit _damageconcussivelightonblock _damageconcussiveheavyonblock _damagetier _cooldowntime _reusetime _selectionweight _knockbackoffensebasic _knockbackoffensespecial _knockbackoffensebasiconblock _knockbackoffensespecialonblock _knockbackdefense _visualstaticmesh _visualskeletalmesh _visualdestructiblemesh _weaponstatusdefault _weaponstatuscurrent _weaponstatusdecrement _perishrate _perishto _maxdurability _repairitem1 _repairitem1_amount _repairitem1_weight _repairitem2 _repairitem2_amount _repairitem2_weight _repairitem3 _repairitem3_amount _repairitem3_weight _affectedbydamagetiers _buildingpiecescore _buildingmaxhealth _repairxp _firstmodifier _secondmodifier _thirdmodifier _fourthmodifier _foodamount _drinkamount _burntime _itemflags _itemcontainersize _avatartype _dyecolourid _warpaintid _staminacostmultiplier _staminaclimbingcostmultiplier _leavesghostitem) (break `ItemTableRow` _returnvalue))
      (bind _object (`|ConvertAsset` _buildingclass))
      (bind _returnvalue_2 (`|SpawnActorFromClass` _object (`SceneComponent.K2_GetComponentToWorld` (`self.StaticMesh`)) "Undefined" "OverrideRootScale" null _templateid false true (`self.OwnerUniqueID`)))
      (bind _returnvalue_3 (`UniqueID.GenerateUniqueID`))
      (`DreamworldBlueprints.SetUniqueID` _returnvalue_2 _returnvalue_3)
      (`PersistenceComponent.SetDirty` (`KismetArrayLibrary.Array_Get` (`self.K2_GetComponentsByClass` _returnvalue_2 "/Script/UE4Dreamworld.ActorPersistenceComponent")) true 5.0)
      ;[1 1 1] Debug
      (bind _name_2 (`/Game/Characters/SurvivalFunctionLibrary.GetNameFromTemplateID` _templateid))
      (bind (_sourceitemtemplateid _isabrush _canbypassbuildingblockervolumes _issnappedtosocket _targetsockettypes _maxhealth _currenthealth _affectedbydamagetiers_2 _claimradiusbuilding _claimradiusfoliage _enforcelandclaim _claimlocation _templateid_2 _requiresforcedghostrefresh _bisstabilitylostdelayed _buildingpiecescore_2 _buildingscore _decaydisabled _decaystate _decaytimestamp) (defaults `/Local/BP_JobBox` _object))
      (`/Game/Systems/BP_MacroGlobal.DebugPrintSimple` (`KismetStringLibrary.Concat_StrStr` (`KismetTextLibrary.Conv_TextToString` _name_2) ": " (`KismetSystemLibrary.GetClassDisplayName` _object) ": GUICategory=" (`|GetEnumeratorNameAsString` _guicategory) " LeavesGhostItem=" (`KismetStringLibrary.Conv_BoolToString` _leavesghostitem) " DecayDisabled=" (`KismetStringLibrary.Conv_BoolToString` _decaydisabled) " DecayState=" (`KismetStringLibrary.Conv_IntToString` _decaystate) " DecayTimestamp=" (`KismetStringLibrary.Conv_DoubleToString` _decaytimestamp) " placeable:" (`KismetStringLibrary.Conv_BoolToString` (`KismetMathLibrary.ClassIsChildOf` _object "/Script/ConanSandbox.PlaceableBase")) " buildable:" (`KismetStringLibrary.Conv_BoolToString` (`KismetMathLibrary.ClassIsChildOf` _object "/Script/ConanSandbox.BuildableBase"))) "INFOL_IMPORTANT" "Modding"
        (:`Output`
          (`ItemInventory.RemoveItem` (`self.PlaceableInventory`) 0)
          (`self.K2_DestroyActor`))))))

(fn `UserConstructionScript`
  (`parent.UserConstructionScript`))